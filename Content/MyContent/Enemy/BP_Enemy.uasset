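; BP_Enemy is an enemy actor that disappears from view when the player's flashlight points at it.
; BeginPlay caches the player pawn, and each Tick compares the flashlight's forward vector with the direction to the enemy by dot product, without range or occlusion checks.
; While lit, the mesh hides after a short Delay; otherwise it shows immediately.
; A Die event plays a sound and destroys the actor.
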(event `self.ReceiveBeginPlay`
  (bind _asbp_example_player (cast `/Game/FPFlashlightAnims/Demo/Player/FirstPerson/Blueprints/BP_ExamplePlayer` (`GameplayStatics.GetPlayerPawn` 0)))
  (set `self.PlayerRef` _asbp_example_player))

(event `Die`
  (`GameplayStatics.PlaySoundAtLocation` null (0.0 0.0 0.0) (struct) 1.0 1.0 0.0 null null null null)
  (`self.K2_DestroyActor`))

(event `self.ReceiveTick`
  (params (DeltaSeconds :type "Float (single-precision)"))
  (bind _playerref (`self.PlayerRef`))
  (bind _spotlight_flashlight (`/Game/FPFlashlightAnims/Demo/Player/FirstPerson/Blueprints/BP_ExamplePlayer.SpotLight_FlashLight` _playerref))
  (`/Engine/EditorBlueprintResources/StandardMacros.IsValid` _playerref
    (:`Is Valid`
      (if (`KismetSystemLibrary.IsValid` _playerref)
        (if (`/Game/FPFlashlightAnims/Demo/Player/FirstPerson/Blueprints/BP_ExamplePlayer.FlashlightUsed?` _playerref)
          (if (> (`KismetMathLibrary.Dot_VectorVector` (`SceneComponent.GetForwardVector` _spotlight_flashlight) (`KismetMathLibrary.Normal` (- (`self.K2_GetActorLocation`) (`SceneComponent.K2_GetComponentLocation` _spotlight_flashlight)))) 0.85)
            (set `self.IsInLight` true)
            (else
              (set `self.IsInLight` false :!label _label)))
          (else
            (goto _label)))
        (if (`self.IsInLight`)
          (`KismetSystemLibrary.Delay` 0.5)
          (`SceneComponent.SetVisibility` (`self.Mesh`) false false)
          (else
            (`SceneComponent.SetVisibility` (`self.Mesh`) true false)))))))

(fn `UserConstructionScript`)